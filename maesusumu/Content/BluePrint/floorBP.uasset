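; Floor tile Blueprint for an endless-runner style track that has the game mode add a new tile as the player leaves this one.
; When ThirdPersonCharacter exits the Box, it calls AddFloorTile on ThirdPersonGameMode and destroys itself two seconds later.
; GetAttachTransform exposes the CreatePoint world location.
; RandomCreate loops over nine spawn points, spawning DamageActor wherever a random roll matches the index, without a fixed count.
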(event OnComponentEndOverlap(Box)
  (params (OverlappedComponent :type Primitive%20Component%20Object%20Reference) (OtherActor :type Actor%20Object%20Reference) (OtherComp :type Primitive%20Component%20Object%20Reference) (OtherBodyIndex :type Integer))
  (Utilities|Casting|CastToThirdPersonCharacter OtherActor)
  (bind _asthird_person_game_mode (Utilities|Casting|CastToThirdPersonGameMode (Game|GetGameMode)))
  (Default|AddFloorTile _asthird_person_game_mode)
  (Utilities|FlowControl|Delay 2.0)
  (Actor|DestroyActor))

(fn ConstructionScript
  (bind _spawnpointarr (Variables|Default|GetspawnPointArr))
  (Utilities|Array|Add _spawnpointarr (Variables|Default|GetspawnPoint1))
  (Utilities|Array|Add _spawnpointarr (Variables|Default|GetspawnPoint2))
  (Utilities|Array|Add _spawnpointarr (Variables|Default|GetspawnPoint3))
  (Utilities|Array|Add _spawnpointarr (Variables|Default|GetspawnPoint4))
  (Utilities|Array|Add _spawnpointarr (Variables|Default|GetspawnPoint5))
  (Utilities|Array|Add _spawnpointarr (Variables|Default|GetspawnPoint6))
  (Utilities|Array|Add _spawnpointarr (Variables|Default|GetspawnPoint7))
  (Utilities|Array|Add _spawnpointarr (Variables|Default|GetspawnPoint8))
  (Utilities|Array|Add _spawnpointarr (Variables|Default|GetspawnPoint9)))

(fn GetAttachTransform
  (return (Transformation|GetWorldLocation (Variables|Default|GetcreatePoint))))

(fn RandomCreate
  (bind (_array_element _array_index) (Utilities|Array|ForEachLoopwithBreak (Variables|Default|GetspawnPointArr))
    (:LoopBody
      (if (== _array_index (Math|Random|RandomIntegerinRange 0 8))
        (Game|SpawnActorfromClass "/Game/BluePrint/damageActor.damageActor_C" (Transformation|GetWorldTransform _array_element) "Undefined" 0 0)))))