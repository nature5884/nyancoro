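; Floor tile actor that keeps a path extending as the player character moves along it, in the style of an endless runner.
; When the ThirdPersonCharacter stops overlapping its Box, the tile tells ThirdPersonGameMode to add a floor tile, then destroys itself after a short delay.
; A CreatePoint component marks an attach point, exposed through GetAttachTransform and cached as CreateLocation during construction.
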(event OnComponentEndOverlap(Box)
  (params (OverlappedComponent :type Primitive%20Component%20Object%20Reference) (OtherActor :type Actor%20Object%20Reference) (OtherComp :type Primitive%20Component%20Object%20Reference) (OtherBodyIndex :type Integer))
  (Utilities|Casting|CastToThirdPersonCharacter OtherActor)
  (bind _asthird_person_game_mode (Utilities|Casting|CastToThirdPersonGameMode (Game|GetGameMode)))
  (Default|AddFloorTile _asthird_person_game_mode)
  (Utilities|FlowControl|Delay 2.0)
  (Actor|DestroyActor))

(fn ConstructionScript
  (Variables|Default|SetcreateLocation (Transformation|GetWorldLocation (Variables|Default|GetcreatePoint))))

(fn GetAttachTransform
  (return (Transformation|GetWorldTransform (Variables|Default|GetcreatePoint))))